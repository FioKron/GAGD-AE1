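; SoundSystem_BP sequences the scripted introduction dialogue between the player, PIBot, the Combat Admin and Sacramento.
; Functions play cues attached to each speaker, with OnAudioFinished bindings chaining many steps and boolean guards preventing most replays.
; It also spawns the Combat Admin and Sacramento, opens name-entry and answer widgets, and changes PIBot's status.
; Player interruptions stop current lines and branch into alternate dialogue; answers select Sacramento's responses.
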(event `InitiatePlayerIntteruptingComAdIntroSequenc`
  (params (OverlappingActor :type "Actor Object Reference"))
  ;[1 1 1] Initilise the alternate introduction dialog sequence for the Combat Admin
  (`self.InitiatePlayerIntteruptingComAdIntroSequence` OverlappingActor))

(event `PIBotIntroDialogStarted`
  ;[1 1 1] Handle PIBot's Introduction
  (add `AudioComponent.OnAudioFinished` (`self.PIBotIntroAskNameAudioComponent`) (delegate `TimeForPlayerToProvideName`)))

(event `TimeForComAd'sIntroductionSequence`
  ;[1 1 1] Handle the Combat Admin's Introduction
  (`self.BeginComAdIntroDialogSequence_BP`)
  (add `AudioComponent.OnAudioFinished` (`self.ComAdIntroDialogCompRef`) (delegate `TimeForPIBotToReplyToComAd'sIntro`)))

(event `InitAltComAdIntroSequence`
  ;[1 1 1] Initilise the alternate introduction dialog sequence for the Combat Admin
  (bind _comadinitintrointteruptdiasequaudcomp (`self.PlayComAdIntroIntteruptInitResponse`))
  (add `AudioComponent.OnAudioFinished` _comadinitintrointteruptdiasequaudcomp (delegate `ComAdIntroInteruptMsgFinished`)))

(event `TimeForPlayerToProvideName`
  ;[1 1 1] Handle PIBot's Introduction
  (`self.ProvideNameToPIBot`))

(event `TimeForPIBotToReplyToComAd'sIntro`
  ;[1 1 1] Handle the Combat Admin's Introduction
  (bind _pibotinitresponsetocomadintroref (`self.PIBotInitReplyToComAdIntroSequence`))
  (add `AudioComponent.OnAudioFinished` _pibotinitresponsetocomadintroref (delegate `TimeForPIBot'sImportantMessageEmphasis`)))

(event `ComAdIntroInteruptMsgFinished`
  ;[1 1 1] When the CombatAdmin has finished their introduction interuption call, have PIBot say a line for such too, then...
  (bind _audcompforpibotimpmsgemphaftercomadintrointter (`self.PlayPIBotImpMsgEmphAfterComAdIntroIntteruption`))
  (add `AudioComponent.OnAudioFinished` _audcompforpibotimpmsgemphaftercomadintrointter (delegate `PIBotImpMsgEmphInterrupted`)))

(event `PlayerHasProvidedName`
  ;[1 1 1] Handle PIBot's Introduction
  (bind _confirmnameaudcompref (`self.RespondToPlayerProvidingName`))
  (add `AudioComponent.OnAudioFinished` _confirmnameaudcompref (delegate `TimeForPIBotToProvideTheirImportantMessage`)))

(event `TimeForPIBot'sImportantMessageEmphasis`
  ;[1 1 1] Handle the Combat Admin's Introduction
  (bind _pibotimpmsgemphaudref (`self.PlayPIBotImportantMessageEmphasis`))
  (add `AudioComponent.OnAudioFinished` _pibotimpmsgemphaudref (delegate `TimeForSacramento'sIntroduction`)))

(event `TimeForSacramento'sIntroduction`
  ;[1 1 1] Handle the Combat Admin's Introduction
  (`self.InitiliseSacramentoSpawnSequence`)
  (bind _sacramentointroaudcompref (`self.PlaySacramentoInitIntroductionMessage`))
  (add `AudioComponent.OnAudioFinished` _sacramentointroaudcompref (delegate `SacramentoInitIntroDialogSegmentComplete`)))

(event `PIBotImpMsgEmphInterrupted`
  ;[1 1 1] ...spawn in Sacramento, to 'interupt' PIBot's attempt at their important message, if the player interupts the CombatAdmin's introduction
  (`self.TimeForSacramento'sIntroduction`))

(event `TimeForPIBotToProvideTheirImportantMessage`
  ;[1 1 1] Handle PIBot's Introduction
  (`self.MentionImportantMessageNotification`))

(event `SacramentoInitIntroDialogSegmentComplete`
  ;[1 1 1] Initiate the Player's response to the first segment of Sacramento's Introduction Dialog
  (`self.SacFirstDialogSegmentComplete`)
  (`self.ProvideAnswerToSacramento'sFirstQuestion`))

(event `PIBotAnswerSacramentoLocationQuestion`
  ;[1 1 1] One potential route in the dialog system
  (`self.PlayPIBotAnswerSacramentoLocationQuestion`))

(fn `BeginComAdIntroDialogSequence_BP`
  ;[1 1 1] When PIBot gets 'interupted', spawn in the CombatAdmin and have them say their introduction dialog lines
  (if (not (`self.ComAdInitIntroSequenceInitiated`))
    (`QuestToBeDefinedCharacter.DisablePlayerCinematicMode` (`self.PlayerInst`))
    (bind _returnvalue (`|SpawnActorFromClass` "/Game/Character/CombatAdmin.CombatAdmin_C" (`KismetMathLibrary.MakeTransform` (15.0 5240.0 1995.0)) "AdjustIfPossibleButDontSpawnIfColliding" "OverrideRootScale"))
    (bind _output_get (set `self.ComAdInst` _returnvalue))
    (bind _returnvalue_2 (`GameplayStatics.SpawnSoundAttached` "/Game/Sound/CombatAdminIntroPH.CombatAdminIntroPH" (`/Game/Character/CombatAdmin.Centre` _output_get)))
    (set `self.ComAdIntroDialogCompRef` _returnvalue_2)
    (set `self.ComAdInitIntroSequenceInitiated` true)))

(fn `HandlePIBotInitIntroductionSequence_BP`
  (params (PIBotReference :type "PIBot Object Reference"))
  (bind _pibotreference (`self.PIBotReference`))
  ;[1 1 1] Call the 'default' version of this function first, as well as initilising other variables
  (bind _playercharacter (`/Game/BlueprintFunctionLibraries/BlueprintCharacterFunctions.GetPlayerCharacter`))
  (set `self.PlayerInst` _playercharacter)
  (bind _output_get (set `self.PIBotInst` PIBotReference))
  (`self.HandlePIBotIntroSequence` _output_get)
  (if (not (`KismetSystemLibrary.IsValid` (`self.PIBotIntroAskNameAudioComponent`)))
    ;[1 1 1] Then handle the initial section of this introduction dialouge sequence
    (if (not (`self.IntroductionAudioInitiated`))
      (bind _returnvalue (`GameplayStatics.SpawnSoundAttached` "/Game/Sound/PIBotIntroAskName_Cue.PIBotIntroAskName_Cue" (`Character.Mesh` _pibotreference) "None" (0.0 0.0 0.0) (struct) "KeepRelativeOffset" false 1.0 1.0 0.0))
      (bind _output_get_2 (set `self.PIBotIntroAskNameAudioComponent` _returnvalue))
      (`BlackboardComponent.SetValueAsObject` (`AIBlueprintHelperLibrary.GetBlackboard` _pibotreference) (`.SelectedKeyName` (break `BlackboardKeySelector` (`self.PIBotIntroAudComp`))) _output_get_2)
      (set `self.IntroductionAudioInitiated` true)
      (`self.PIBotIntroDialogStarted`))
    (else
      (`self.TurnToFacePlayer`))))

(fn `HandlePIBotIntroInterrupted_BP`
  ;[1 1 1] Call the functions for interrupting PIBot's introduction, only if PIBot's introduction was interrupted
  (`AudioComponent.Stop` (`self.PIBotIntroAskNameAudioComponent`))
  (bind _returnvalue (`GameplayStatics.SpawnSoundAttached` "/Game/Sound/PIBotIntroInterupted_Cue.PIBotIntroInterupted_Cue" (`Character.Mesh` (`self.PIBotInst`))))
  (set `self.HeyWaitAudioCompRef` _returnvalue)
  (`self.ProvideNameToPIBot`))

(fn `HaveSacramentoRespondToFirstQuestionAnswer`
  (params (PlayersAnswer :type String))
  (returns (SacResponseAudioComp :type "AudioComponent Object Reference"))
  (bind _sacramentoinst (`self.SacramentoInst`))
  (bind _mesh (`Character.Mesh` _sacramentoinst))
  ;[1 1 1] Handle Sacramento's response to the answer provided by the Player to the first question that Sacramento asked of them
  (bind _returnvalue (`Sacramento.GetPlayersFirstIntroQuestionAnswer` (`self.SacramentoInst`) PlayersAnswer))
  (switch `string` _returnvalue
    (:`No where in particular`
      (`/Game/Character/SacramentoBlueprint.IsPIBotResponseToIntroPlaying?` _sacramentoinst)
      (bind _returnvalue_2 (`GameplayStatics.SpawnSoundAttached` "/Game/Sound/SacramentoResponseToNowhereInParticular_Cue.SacramentoResponseToNowhereInParticular_Cue" _mesh))
      (set `self.SacResponseAudioComp` _returnvalue_2)
      (return (stale _output_get)))
    (:`I am waiting for this robot to tell me`
      (`/Game/Character/SacramentoBlueprint.IsPIBotResponseToIntroPlaying?` _sacramentoinst)
      (bind _returnvalue_3 (`GameplayStatics.SpawnSoundAttached` "/Game/Sound/SacramentoResponseToIAmWaitingForThisRobotToTellMe_Cue.SacramentoResponseToIAmWaitingForThisRobotToTellMe_Cue" _mesh))
      (bind _output_get (set `self.SacResponseAudioComp` _returnvalue_3))
      (return _output_get))
    (:`I do not know...`
      (`/Game/Character/SacramentoBlueprint.IsPIBotResponseToIntroPlaying?` _sacramentoinst)
      (bind _returnvalue_4 (`GameplayStatics.SpawnSoundAttached` "/Game/Sound/SacramentosResponseToIDonotKnow_Cue.SacramentosResponseToIDonotKnow_Cue" _mesh))
      (set `self.SacResponseAudioComp` _returnvalue_4)
      (return _output_get))
    (:`Answer of no effect`
      (`KismetSystemLibrary.PrintString` "'Answer of no effect' is the answer the player gave"))))

(fn `InitiatePlayerIntteruptingComAdIntroSequence`
  (params (OverlappingActor :type "Actor Object Reference"))
  ;[1 1 1] If the player reaches this trigger before ComAd finishes their intro sequence, tell ComAd to stop their intro sequence
  (if (not (`QuestToBeDefinedCharacter.bPlayerInteruptedComAdIntro` (stale _asquest_to_be_defined_character)))
    (bind _asquest_to_be_defined_character (cast `QuestToBeDefinedCharacter` OverlappingActor))
    (if (not (`QuestToBeDefinedCharacter.bPlayerInteruptedComAdIntro` _asquest_to_be_defined_character))
      (if (not (`self.ClearedUpExistingInst`))
        (bind _outactors (`GameplayStatics.GetAllActorsOfClass` "/Game/Character/SacramentoBlueprint.SacramentoBlueprint_C"))
        (for _array_element _outactors
          (`self.K2_DestroyActor` _array_element))
        (set `self.ClearedUpExistingInst` true))
      (bind _combatadmininst (`/Game/BlueprintFunctionLibraries/BlueprintCharacterFunctions.GetCombatAdmin`))
      (bind _output_get (set `self.ComAdInst` _combatadmininst))
      (`/Game/Character/CombatAdmin.IntroInterupted` _output_get)
      (if (`/Game/Character/CombatAdmin.HasIntroBeenInterupted` _output_get)
        (`self.InitAltComAdIntroSequence`)))))

(fn `InitiliseSacramentoSpawnSequence`
  ;[1 1 1] Handle Spawning Sacramento into the level
  (bind _outactors (`GameplayStatics.GetAllActorsOfClass` "/Game/Blueprints/Actors/SacramentoSlugShotgun.SacramentoSlugShotgun_C"))
  (bind _sacramento (`/Game/BlueprintFunctionLibraries/BlueprintCharacterFunctions.SpawnInSacramento` (3090.0 7250.0 160.0) (0.0 0.0 0.0) (`KismetArrayLibrary.Array_Get` _outactors)))
  (set `self.SacramentoInst` _sacramento))

(fn `MentionImportantMessageNotification`
  (bind _pibotinst (`self.PIBotInst`))
  ;[1 1 1] Handle PIBot's Important Message notification
  (if (not (`self.PIBotHasProvidedImportantMessageNotification`))
    (bind _aspibot_blueprint (cast `/Game/Character/PIBotBlueprint` (`self.PIBotInst`)))
    (bind _pibotwilltellplayersomethingsoonaudcomp (`/Game/Character/PIBotBlueprint.PlayPIBotWillTellPlayerSomethingSoonCue` _aspibot_blueprint))
    (bind _output_get (set `self.TellPlayerSomethingSoonAudioCompRef` _pibotwilltellplayersomethingsoonaudcomp))
    (set `PIBot.DialogLinesAfterIntro` _output_get _pibotinst)
    (`QuestToBeDefinedCharacter.DisablePlayerCinematicMode` (`self.PlayerInst`))
    (set `PIBot.CurrentStatus` "PS_IdleDead" _pibotinst)
    (`Widget.RemoveFromParent` (`self.NameEntryWidget`))
    (set `self.PIBotHasProvidedImportantMessageNotification` true)))

(fn `PIBotInitReplyToComAdIntroSequence`
  (returns (PIBotInitResponseToComAdIntroRef :type "AudioComponent Object Reference"))
  (bind _pibotinst (`self.PIBotInst`))
  ;[1 1 1] Play PIBot's response to the CombatAdmin's introduction when they have finished
  (if (`PIBot.bComAdIntroHasBeenInterupted` _pibotinst)
    _
    (elif (not (`self.PIBotInitResponseToComAdIntroStarted`))
      (bind _returnvalue (`GameplayStatics.SpawnSoundAttached` "/Game/Sound/PIBotResponseToComAdIntro_Cue.PIBotResponseToComAdIntro_Cue" (`Character.Mesh` _pibotinst)))
      (bind _output_get (set `self.PIBotResponseToComAdIntro` _returnvalue))
      (set `self.PIBotInitResponseToComAdIntroStarted` true)
      (return _output_get))))

(fn `PlayComAdIntroIntteruptInitResponse`
  (returns (ComAdInitIntroIntteruptDiaSequAudComp :type "AudioComponent Object Reference"))
  ;[1 1 1] If the CombatAdmin's introduction has been interupted by the player, have the ComAd call out to the Player
  (`PIBot.ComAdIntroInterupted` (`self.PIBotInst`))
  (if (not (`self.ComAdIntroInteruptionDialogSeqenceStarted`))
    (`AudioComponent.Stop` (`self.PIBotResponseToComAdIntro`))
    (`AudioComponent.Stop` (`self.PIBotImpMsgEmphasis`))
    (`AudioComponent.Stop` (`self.ComAdIntroDialogCompRef`))
    (bind _returnvalue (`GameplayStatics.SpawnSoundAttached` "/Game/Sound/CombatAdminIntroInteruptedPH_Cue.CombatAdminIntroInteruptedPH_Cue" (`/Game/Character/CombatAdmin.Centre` (`self.ComAdInst`))))
    (set `self.ComAdIntroInteruptionDialogSeqenceStarted` true)
    (return _returnvalue)))

(fn `PlayerDoesNotMindStaying`
  ;[1 1 1] Play this response to the answer the Player has provided/had chosen for them, at this point
  (`GameplayStatics.SpawnSoundAttached` "/Game/Sound/PlayerDoesNotMindStayingFullResponse_Cue.PlayerDoesNotMindStayingFullResponse_Cue" (`Character.Mesh` (`self.SacramentoInst`))))

(fn `PlayerWouldMindStaying`
  (returns (PlayerWillMindStayingAudComp :type "AudioComponent Object Reference"))
  ;[1 1 1] Play this response to the answer the Player has provided/had chosen for them, at this point
  (bind _returnvalue (`GameplayStatics.SpawnSoundAttached` "/Game/Sound/SacramentoPlayerDoesMindStaying_Cue.SacramentoPlayerDoesMindStaying_Cue" (`Character.Mesh` (`self.SacramentoInst`))))
  (return _returnvalue))

(fn `PlayPIBotAnswerSacramentoLocationQuestion`
  (returns (PIBotResponseToDestinationQuestion :type "AudioComponent Object Reference"))
  (bind _pibotinst (`self.PIBotInst`))
  ;[1 1 1] Have PIBot reappear and say the dialog piece for this route
  (set `PIBot.CurrentStatus` "PS_HarmlessFollowingPlayer" _pibotinst)
  (bind _returnvalue (`GameplayStatics.SpawnSoundAttached` "/Game/Sound/PIBotResponseToSacramentoDestinationQuestionFinal_Cue.PIBotResponseToSacramentoDestinationQuestionFinal_Cue" (`Character.Mesh` _pibotinst)))
  (return _returnvalue))

(fn `PlayPIBotImpMsgEmphAfterComAdIntroIntteruption`
  (returns (AudCompForPIBotImpMsgEmphAfterComAdIntroIntter :type "AudioComponent Object Reference"))
  ;[1 1 1] Play PIBot's response to the Combat Admin's response, for having their introduction interupted
  (if (not (`self.PIBotImpMsgEmphAfterComAdIntterStarted`))
    (bind _returnvalue (`GameplayStatics.SpawnSoundAttached` "/Game/Sound/PIBotImportantMessageEmphasisAfterComAdIntroInterupt_Cue.PIBotImportantMessageEmphasisAfterComAdIntroInterupt_Cue" (`Character.Mesh` (`self.PIBotInst`))))
    (return _returnvalue)))

(fn `PlayPIBotImportantMessageEmphasis`
  (returns (PIBotImpMsgEmphAudRef :type "AudioComponent Object Reference"))
  (bind _pibotinst (`self.PIBotInst`))
  ;[1 1 1] Then player have PIBot emphasise their important message again
  (if (`PIBot.bComAdIntroHasBeenInterupted` _pibotinst)
    _
    (elif (not (`self.PIBotImpMsgEmphInitiated`))
      (bind _returnvalue (`GameplayStatics.SpawnSoundAttached` "/Game/Sound/PIBotImportantMessageEmphasis_Cue.PIBotImportantMessageEmphasis_Cue" (`Character.Mesh` _pibotinst)))
      (bind _output_get (set `self.PIBotImpMsgEmphasis` _returnvalue))
      (return _output_get))))

(fn `PlaySacramentoInitIntroductionMessage`
  (returns (SacramentoIntroAudCompRef :type "AudioComponent Object Reference"))
  ;[1 1 1] Handle Sacramento's opening segment for his introduction
  (bind _returnvalue (`GameplayStatics.SpawnSoundAttached` "/Game/Sound/SacramentoFirstIntroSectionDialog_Cue.SacramentoFirstIntroSectionDialog_Cue" (`Character.Mesh` (`self.SacramentoInst`))))
  (return _returnvalue))

(fn `ProvideAnswerToSacramento'sFirstQuestion`
  ;[1 1 1] Initilise creation of this widget for the Player to use
  (bind _returnvalue (`|CreateWidget` "/Game/Blueprints/PlayerHUDElements/SacramentoFirstQuestionAnswer.SacramentoFirstQuestionAnswer_C"))
  (bind _output_get (set `self.SacramentoFirstQuestionAnswerWidget` _returnvalue))
  (`UserWidget.AddToPlayerScreen` _output_get 0))

(fn `ProvideNameToPIBot`
  (bind _playerinst (`self.PlayerInst`))
  ;[1 1 1] Only create the respective widget, if it has not already been created
  (if (not (`self.NameEntryWidgetCreated`))
    (`QuestToBeDefinedCharacter.InteruptPIBotIntro` _playerinst)
    (bind _nameinputwidgetref (`/Game/Blueprints/MyCharacter.InitPlayerNameSet` _playerinst))
    (set `self.NameEntryWidget` _nameinputwidgetref)
    (`QuestToBeDefinedCharacter.EnablePlayerCinematicMode` _playerinst)
    (set `self.NameEntryWidgetCreated` true)))

(fn `RespondToPlayerProvidingName`
  (returns (ConfirmNameAudCompRef :type "AudioComponent Object Reference"))
  (bind _pibotinst (`self.PIBotInst`))
  ;[1 1 1] When the player has confirmed (or has not), what their name is, have PIBot give their response if they have not already, then when the associated cue finishes, remove the name entry widget from its parent, play another cue for PIBot, disable player cinematic mode, then finish execution for this task
  (if (not (`self.PIBotAlreadyGivenResponse`))
    (`PIBot.BeginPIBotIntroSequence` _pibotinst)
    (bind _aspibot_blueprint (cast `/Game/Character/PIBotBlueprint` _pibotinst))
    (bind _confirmnameaudcompref (`/Game/Character/PIBotBlueprint.RespondToPlayerCharsNameChoice` _aspibot_blueprint (`self.HeyWaitAudioCompRef`)))
    (return _confirmnameaudcompref)))

(fn `SacFirstDialogSegmentComplete`
  (bind _pibotinst (`self.PIBotInst`))
  ;[1 1 1] When Sacramento has finished their first dialog section, have PIBot hide out of sight from Sacramento (as well as from the Player)
  (`PIBot.PIBotNowSeenSacramentoFirstTime` _pibotinst)
  (set `PIBot.CurrentStatus` "PS_Hide" _pibotinst))

(fn `TurnToFacePlayer`
  (bind _pibotinst (`self.PIBotInst`))
  ;[1 1 1] Rotate PIBot to face the PlayerCharacter, only perform rotation in Yaw though
  (`self.K2_SetActorRotation` _pibotinst (`KismetMathLibrary.MakeRotator` 0.0 0.0 (.yaw (`KismetMathLibrary.FindLookAtRotation` (`self.K2_GetActorLocation` _pibotinst) (`self.K2_GetActorLocation` (`self.PlayerInst`))))) false))

(fn `UserConstructionScript`)